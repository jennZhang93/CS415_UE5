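; BP_Bullet is a projectile actor that flies at an adjustable speed and destroys itself on impact.
; Tick sweeps the Bullet component along world X by BulletSpeed times delta time, and ChangeBulletSpeed sets that speed.
; The hit check compares the other actor's display name with itself, so it does not filter by target.
; Unconnected InitialSpeed and MaxSpeed setters never run.
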(event `ChangeBulletSpeed`
  (params (NewSpeed :type "Float (double-precision)"))
  (set `self.BulletSpeed` NewSpeed))

(event `self.ReceiveTick`
  (params (DeltaSeconds :type "Float (single-precision)"))
  (`SceneComponent.K2_AddWorldOffset` (`self.Bullet`) (`KismetMathLibrary.MakeVector` (* DeltaSeconds (`self.BulletSpeed`))) true false))

(event `self.Bullet.OnComponentHit`
  (params (HitComponent :type "PrimitiveComponent Object Reference") (OtherActor :type "Actor Object Reference") (OtherComp :type "PrimitiveComponent Object Reference") (NormalImpulse :type "Vector Structure") (Hit :type "HitResult Structure (by ref)"))
  (bind _returnvalue (`KismetSystemLibrary.GetDisplayName` OtherActor))
  (if (`KismetStringLibrary.Contains` _returnvalue _returnvalue)
    (`self.K2_DestroyActor`)))

(fn `UserConstructionScript`)