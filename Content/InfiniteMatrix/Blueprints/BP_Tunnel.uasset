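; BP_Tunnel is a tunnel segment with a rotating wall, a randomly placed enemy and four health packs.
; Passing its trigger awards the player a point; hitting the wall costs health, and both destroy the segment and request a replacement from TunnelSpawner.
; The wall also destroys bullets, and health packs heal on hit.
; RandomizeWall picks one of four hole meshes and a random roll, but is not called here.
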(event `self.ReceiveBeginPlay`
  ;[1 1 1] Spawn Enemy
  (`|SpawnActorFromClass` "/Game/InfiniteMatrix/Blueprints/BP_Enemy.BP_Enemy_C" (`KismetMathLibrary.MakeTransform` (`SceneComponent.K2_GetComponentLocation` (`|GetArrayItem` (`|MakeArray` (`self.Enemy3`) (`self.Enemy2`) (`self.Enemy1`) (`self.Enemy4`) (`self.Enemy5`) (`self.Enemy6`)) (`KismetMathLibrary.RandomInteger` 6)))) "Undefined" "OverrideRootScale" null null))

(event `self.ReceiveTick`
  (params (DeltaSeconds :type "Float (single-precision)"))
  (`SceneComponent.K2_AddLocalRotation` (`self.WallMesh`) (`KismetMathLibrary.MakeRotator` (* DeltaSeconds (`self.RotateSpeed`))) false false))

(event `self.TriggerZone.OnComponentBeginOverlap`
  (params (OverlappedComponent :type "PrimitiveComponent Object Reference") (OtherActor :type "Actor Object Reference") (OtherComp :type "PrimitiveComponent Object Reference") (OtherBodyIndex :type Integer) (bFromSweep :type Boolean) (SweepResult :type "HitResult Structure (by ref)"))
  (bind _asbp_player (cast `/Game/InfiniteMatrix/Blueprints/BP_Player` OtherActor))
  (`/Game/InfiniteMatrix/Blueprints/BP_Player.IncreasePoint` _asbp_player 1)
  (`/Game/InfiniteMatrix/Blueprints/BP_TunnelSpawner.SpawnTunnelAtSpawnPoint` (`self.TunnelSpawner`))
  (`self.K2_DestroyActor`))

(event `self.WallMesh.OnComponentHit`
  (params (HitComponent :type "PrimitiveComponent Object Reference") (OtherActor :type "Actor Object Reference") (OtherComp :type "PrimitiveComponent Object Reference") (NormalImpulse :type "Vector Structure") (Hit :type "HitResult Structure (by ref)"))
  (`|ExecutionSequence`
    (:`then_0`
      (bind _asbp_bullet (cast `/Game/InfiniteMatrix/Blueprints/BP_Bullet` OtherActor))
      (`self.K2_DestroyActor` _asbp_bullet))
    (:`then_1`
      (bind _asbp_player (cast `/Game/InfiniteMatrix/Blueprints/BP_Player` OtherActor))
      (`|ExecutionSequence`
        (:`then_0`
          (`self.K2_DestroyActor`) ; 1. destroy current tunnel if hit player
        )
        (:`then_1`
          (`/Game/InfiniteMatrix/Blueprints/BP_TunnelSpawner.SpawnTunnelAtSpawnPoint` (`self.TunnelSpawner`)) ; 2. spawn new tunnel
        )
        (:`then_2`
          (`/Game/InfiniteMatrix/Blueprints/BP_Player.DecreaseHealth` _asbp_player 20.0))))))

(event `self.HealthPack1.OnComponentHit`
  (params (HitComponent :type "PrimitiveComponent Object Reference") (OtherActor :type "Actor Object Reference") (OtherComp :type "PrimitiveComponent Object Reference") (NormalImpulse :type "Vector Structure") (Hit :type "HitResult Structure (by ref)"))
  ;[1 1 1] Health pack system
  (bind _asbp_player (cast `/Game/InfiniteMatrix/Blueprints/BP_Player` OtherActor))
  (`/Game/InfiniteMatrix/Blueprints/BP_Player.IncreaseHealth` _asbp_player 10.0)
  (`ActorComponent.K2_DestroyComponent` (`self.HealthPack1`)))

(event `DestroyHealthPack1`
  ;[1 1 1] Health pack system
  (`ActorComponent.K2_DestroyComponent` (`self.HealthPack1`)))

(event `self.HealthPack2.OnComponentHit`
  (params (HitComponent :type "PrimitiveComponent Object Reference") (OtherActor :type "Actor Object Reference") (OtherComp :type "PrimitiveComponent Object Reference") (NormalImpulse :type "Vector Structure") (Hit :type "HitResult Structure (by ref)"))
  ;[1 1 1] Health pack system
  (bind _asbp_player (cast `/Game/InfiniteMatrix/Blueprints/BP_Player` OtherActor))
  (`/Game/InfiniteMatrix/Blueprints/BP_Player.IncreaseHealth` _asbp_player 10.0)
  (`ActorComponent.K2_DestroyComponent` (`self.HealthPack2`)))

(event `DestroyHealthPack2`
  ;[1 1 1] Health pack system
  (`ActorComponent.K2_DestroyComponent` (`self.HealthPack2`)))

(event `self.HealthPack3.OnComponentHit`
  (params (HitComponent :type "PrimitiveComponent Object Reference") (OtherActor :type "Actor Object Reference") (OtherComp :type "PrimitiveComponent Object Reference") (NormalImpulse :type "Vector Structure") (Hit :type "HitResult Structure (by ref)"))
  ;[1 1 1] Health pack system
  (bind _asbp_player (cast `/Game/InfiniteMatrix/Blueprints/BP_Player` OtherActor))
  (`/Game/InfiniteMatrix/Blueprints/BP_Player.IncreaseHealth` _asbp_player 10.0)
  (`ActorComponent.K2_DestroyComponent` (`self.HealthPack3`)))

(event `DestroyHealthPack3`
  ;[1 1 1] Health pack system
  (`ActorComponent.K2_DestroyComponent` (`self.HealthPack3`)))

(event `self.HealthPack4.OnComponentHit`
  (params (HitComponent :type "PrimitiveComponent Object Reference") (OtherActor :type "Actor Object Reference") (OtherComp :type "PrimitiveComponent Object Reference") (NormalImpulse :type "Vector Structure") (Hit :type "HitResult Structure (by ref)"))
  ;[1 1 1] Health pack system
  (bind _asbp_player (cast `/Game/InfiniteMatrix/Blueprints/BP_Player` OtherActor))
  (`/Game/InfiniteMatrix/Blueprints/BP_Player.IncreaseHealth` _asbp_player 10.0)
  (`ActorComponent.K2_DestroyComponent` (`self.HealthPack4`)))

(event `DestroyHealthPack4`
  ;[1 1 1] Health pack system
  (`ActorComponent.K2_DestroyComponent` (`self.HealthPack4`)))

(fn `RandomizeWall`
  (`StaticMeshComponent.SetStaticMesh` (`self.WallMesh`) (select `int` (`KismetMathLibrary.RandomIntegerInRange` 0 3) :`0` "/Game/InfiniteMatrix/Meshes/SM_Hole_01.SM_Hole_01" :`1` "/Game/InfiniteMatrix/Meshes/SM_Hole_02.SM_Hole_02" :`2` "/Game/InfiniteMatrix/Meshes/SM_Hole_03.SM_Hole_03" :`3` "/Game/InfiniteMatrix/Meshes/SM_Hole_04.SM_Hole_04" :!type "StaticMesh Object Reference"))
  (`SceneComponent.K2_AddLocalRotation` (`self.WallMesh`) (`KismetMathLibrary.MakeRotator` (`KismetMathLibrary.RandomFloatInRange` 0.0 360.0)) false false))

(fn `UserConstructionScript`)